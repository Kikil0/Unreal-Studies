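; BP_FenceSpline is a construction-script tool that lays a fence along a spline, with no active runtime logic.
; It divides the spline by Length and adds an X-forward spline mesh per segment, positioned from the spline's local-space points.
; Start tangents are clamped to Length, while end tangents are clamped to zero.
; Unseeded random pitch offsets are applied to each new mesh's child component at index 2 on every construction run.
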(event EventBeginPlay)

(event Collision|EventActorBeginOverlap
  (params (OtherActor :type Actor%20Object%20Reference)))

(event EventTick
  (params (DeltaSeconds :type Float%20%28single-precision%29)))

(fn ConstructionScript
  (bind _spline (Variables|Default|GetSpline))
  (bind _length (Variables|Default|GetLength))
  (for _index (range 0 (Math|Float|Truncate (/ (Spline|GetSplineLength (Variables|Default|GetSpline)) (Variables|Default|GetLength))))
    (bind _returnvalue (AddComponent|AddSplineMeshComponent false))
    (SplineMesh|SetForwardAxis _returnvalue "X" true)
    (Transformation|SetRelativeRotation (Components|GetChildComponent _returnvalue 2) (Math|Rotator|MakeRotator 0.0 (+ (.pitch (Variables|/Script/Engine.SceneComponent|GetRelativeRotation (Components|GetChildComponent _returnvalue 2))) (Math|Random|RandomFloatinRange -1e+01 1e+01)) 0.0) false false)
    (SplineMesh|SetStartandEnd _returnvalue (Spline|GetLocationatDistanceAlongSpline _spline (* _index _length) "Local") (Math|Vector|ClampVectorSize (Spline|GetTangentatDistanceAlongSpline _spline (* _index _length) "Local") 0.0 _length) (Spline|GetLocationatDistanceAlongSpline _spline (* (+ _index 1) _length) "Local") (Math|Vector|ClampVectorSize (Spline|GetTangentatDistanceAlongSpline _spline (* (+ _index 1) _length) "Local") 0.0 0.0) true :!class /Script/Engine.SplineMeshComponent)))